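; BP_Heroe is the first-person player character, with move, look, jump, toggled run and shooting.
; On BeginPlay it spawns a BP_Rifle, attaches it, and fires it along the camera's forward vector while the shoot axis is fully held.
; Any actor overlap grants triple jump on a timer counted down in Tick frames rather than seconds, then restores single jump.
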(event EventBeginPlay
  (bind _returnvalue (Game|SpawnActorfromClass "/Game/Objects/Guns/machinegun/BP_Rifle.BP_Rifle_C" (Math|Transform|MakeTransform "0, 0, 0") "Undefined" 0 0))
  (bind _output_get (Variables|Default|SetEquippedGun _returnvalue))
  (Transformation|AttachComponentToComponent _output_get (Variables|Default|GetPersonalGunLocation) "None" "KeepRelative" "KeepRelative" "KeepRelative" true))

(event Collision|EventActorBeginOverlap
  (params (OtherActor :type Actor%20Object%20Reference))
  (Variables|Default|SetJumpMaxCount 3)
  (Variables|Default|SetT_JumpTimer 180))

(event EventTick
  (params (DeltaSeconds :type Float%20%28single-precision%29))
  (if (> (Variables|Default|GetT_JumpTimer) 0)
    (bind _output_get (Variables|Default|SetT_JumpTimer (- (Variables|Default|GetT_JumpTimer) 1)))
    (if (<= _output_get 0)
      (Variables|Default|SetJumpMaxCount 1))))

(event Input|ActionEvents|InputActionA_jump
  (params (Key :type Key%20Structure :default "None"))
  (:Pressed
    (Character|Jump))
  (:Released
    (Character|StopJumping)))

(event Input|ActionEvents|InputActionA_Run
  (params (Key :type Key%20Structure :default "None"))
  (bind _charactermovement (Variables|Character|GetCharacterMovement))
  (:Pressed
    (if (Variables|Default|GetT_Run)
      (Variables|Default|SetT_Run false)
      (Variables|/Script/Engine.CharacterMovementComponent|SetMaxWalkSpeed _charactermovement 6e+02)
      (else
        (Variables|Default|SetT_Run true)
        (Variables|/Script/Engine.CharacterMovementComponent|SetMaxWalkSpeed _charactermovement 1e+03)))))

(event Input|AxisEvents|InputAxisM_Forward
  (params (AxisValue :type Float%20%28single-precision%29))
  (Pawn|Input|AddMovementInput (Transformation|GetActorForwardVector) AxisValue false))

(event Input|AxisEvents|InputAxisM_Right
  (params (AxisValue :type Float%20%28single-precision%29))
  (Pawn|Input|AddMovementInput (Transformation|GetActorRightVector) AxisValue false))

(event Input|AxisEvents|InputAxisM_Shoot
  (params (AxisValue :type Float%20%28single-precision%29))
  (bind _fpscamera (Variables|Default|GetFPSCamera))
  (bind _returnvalue (Transformation|GetWorldLocation _fpscamera))
  (if (Math|Float|NearlyEqual(Float) AxisValue 1.0 1e-06)
    (Default|Shoot (Variables|Default|GetEquippedGun) _returnvalue (+ _returnvalue (* (Math|Vector|GetForwardVector _fpscamera) (Variables|/Game/Objects/Guns/BP_BaseGun.BP_BaseGun_C|GetBulletDistance (Variables|Default|GetEquippedGun)))))))

(event Input|AxisEvents|InputAxisM_Yaw
  (params (AxisValue :type Float%20%28single-precision%29))
  (Pawn|Input|AddControllerYawInput AxisValue))

(event Input|AxisEvents|InputAxisM_Pitch
  (params (AxisValue :type Float%20%28single-precision%29))
  (Pawn|Input|AddControllerPitchInput (* AxisValue -1.0)))

(fn ConstructionScript
  (Variables|Default|SetJumpMaxCount 1)
  (Variables|Default|SetJumpMaxHoldTime 0.0)
  (Variables|Default|SetT_Run false))