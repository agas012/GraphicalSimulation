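; BP_Target is a damageable target that changes emissive color as it loses health and disappears when health runs out.
; BeginPlay creates a dynamic material instance, stores its default color and calls Reset.
; AnyDamage feeds TakeDamage, which lowers clamped health, blends the color toward DamagedColor, and at zero hides the mesh and disables collision.
; Reset restores health, color, visibility and collision, so the actor is reused rather than destroyed.
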(event EventBeginPlay
  (bind _returnvalue (Rendering|Material|CreateDynamicMaterialInstance "/Game/Materials/Surface/M_target_Inst.M_target_Inst" "None" :!class /Script/Engine.KismetMaterialLibrary))
  (bind _output_get (Variables|Default|SetM_Target_DI _returnvalue))
  (Rendering|Material|SetMaterial (Variables|Default|GetTargetMesh) 0 _output_get)
  (bind _returnvalue_2 (Rendering|Material|GetVectorParameterValue (Variables|Default|GetM_Target_DI) "EmissiveColor" :!class /Script/Engine.MaterialInstanceDynamic))
  (Variables|Default|SetDefaultColor _returnvalue_2)
  (CallFunction|Reset))

(event Collision|EventActorBeginOverlap
  (params (OtherActor :type Actor%20Object%20Reference)))

(event EventTick
  (params (DeltaSeconds :type Float%20%28single-precision%29)))

(event Game|Damage|EventAnyDamage
  (params (Damage :type Float%20%28single-precision%29) (DamageType :type Damage%20Type%20Object%20Reference) (InstigatedBy :type Controller%20Object%20Reference) (DamageCauser :type Actor%20Object%20Reference))
  (CallFunction|TakeDamage Damage))

(fn ConstructionScript)

(fn UpdateColor
  (Rendering|Material|SetVectorParameterValue (Variables|Default|GetM_Target_DI) "EmissiveColor" (Math|Color|Lerp(LinearColor) (Variables|Default|GetDamagedColor) (Variables|Default|GetDefaultColor) (Math|Float|Clamp(Float) (/ (Variables|Default|GetHealth) (Variables|Default|GetMaxHealth)))) :!class /Script/Engine.MaterialInstanceDynamic))

(fn Reset
  (Variables|Default|SetHealth (Variables|Default|GetMaxHealth))
  (CallFunction|UpdateColor)
  (Rendering|SetVisibility (Variables|Default|GetTargetMesh) true false)
  (Collision|SetCollisionEnabled (Variables|Default|GetTargetMesh) "QueryAndPhysics"))

(fn TakeDamage
  (params (Damage :type Float%20%28single-precision%29))
  (bind _targetmesh (Variables|Default|GetTargetMesh))
  (bind _output_get (Variables|Default|SetHealth (Math|Float|Clamp(Float) (- (Variables|Default|GetHealth) Damage) 0.0 (Variables|Default|GetMaxHealth))))
  (CallFunction|UpdateColor)
  (if (== _output_get 0.0)
    (Rendering|SetVisibility _targetmesh false false)
    (Collision|SetCollisionEnabled _targetmesh "NoCollision")))